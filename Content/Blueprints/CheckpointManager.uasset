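; CheckpointManager runs a lap-based checkpoint course, timing laps and counting completed ones.
; On BeginPlay it indexes its Checkpoints array, binds each checkpoint's cleared event and activates the first.
; Each clear activates the next checkpoint in order, and clearing the first starts the lap timer.
; Clearing the last records and prints the lap time, calls LapCompleted, then restarts the sequence until TotalLaps is reached.
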(event EventBeginPlay
  (bind _checkpoints (Variables|Default|GetCheckpoints))
  (for (_array_element _array_index) _checkpoints
    (Variables|/Game/Blueprints/Checkpoint.Checkpoint_C|SetCheckpointIndex _array_element _array_index)
    (EventDispatchers|BindEventtoCheckpointCleared _array_element (EventDispatchers|CreateEvent :!event CheckpointCleared)))
  (CallFunction|ActivateCheckpoint (Utilities|Array|Get(acopy) _checkpoints)))

(fn ConstructionScript)

(fn ActivateCheckpoint
  (params (checkpoint :type Checkpoint%20Object%20Reference))
  (Default|SetasActive checkpoint))

(fn CheckpointCleared
  (params (Checkpoint :type Checkpoint%20Object%20Reference))
  (bind _checkpointindex (Variables|/Game/Blueprints/Checkpoint.Checkpoint_C|GetCheckpointIndex Checkpoint))
  (if (== _checkpointindex 0)
    (Variables|Default|SetStartTime (Utilities|Time|GetTimeSeconds)))
  (if (< _checkpointindex (- (Utilities|Array|Length (Variables|Default|GetCheckpoints)) 1))
    (CallFunction|ActivateCheckpoint (Utilities|Array|Get(acopy) (Variables|Default|GetCheckpoints) (+ _checkpointindex 1)))
    (else
      (Utilities|Array|Add (Variables|Default|GetLapTimes) (- (Utilities|Time|GetTimeSeconds) (Variables|Default|GetStartTime)))
      (bind _result (Math|Integer|IncrementInt (Variables|Default|GetCompletedLaps))
        (:%20%20
          (Development|PrintString (Utilities|String|ToString(Float) (- (Utilities|Time|GetTimeSeconds) (Variables|Default|GetStartTime))))
          (Default|CallLapCompleted (- (Utilities|Time|GetTimeSeconds) (Variables|Default|GetStartTime)))
          (if (not (== _result (Variables|Default|GetTotalLaps)))
            (CallFunction|ActivateCheckpoint (Utilities|Array|Get(acopy) (Variables|Default|GetCheckpoints)))
            (Variables|Default|SetStartTime (Utilities|Time|GetTimeSeconds))))))))