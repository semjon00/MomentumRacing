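; Checkpoint actor that the player ship clears by passing through it while it is active.
; SetAsActive turns it on and shows its marker mesh.
; When the ship's overlap ends, a dot product of velocity and the arrow's forward vector rejects backward passes, unless the checkpoint is double-sided.
; A valid pass deactivates it, hides the marker and calls CheckpointCleared with itself; particle shutdown nodes are unconnected.
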(event Collision|EventActorEndOverlap
  (params (OtherActor :type Actor%20Object%20Reference))
  (if (Math|Boolean|Equal(Boolean) (Variables|CustomVariables|GetIsActive) true)
    (bind _asplayer_ship_bp (Utilities|Casting|CastToPlayerShipBP OtherActor))
    (if (or (>= (Math|Vector|DotProduct (Transformation|GetVelocity _asplayer_ship_bp) (Math|Rotator|GetRotationXVector (Transformation|GetWorldRotation (Variables|Default|GetArrow)))) 0.0) (Variables|Default|GetIsDoubleSided))
      (Variables|CustomVariables|SetIsActive false)
      (Rendering|SetVisibility (Variables|Default|GetMarkerMesh) false false)
      (Default|CallCheckpointCleared self))))

(fn ConstructionScript)

(fn SetasActive
  (Development|PrintString "Checkpoint set as active")
  (Variables|CustomVariables|SetIsActive true)
  (Rendering|SetVisibility (Variables|Default|GetMarkerMesh) true false))