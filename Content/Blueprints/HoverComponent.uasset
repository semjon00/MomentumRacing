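; HoverComponent is a component that makes a physics-simulated mesh hover above surfaces, acting as a spring-damper at its own location.
; InitComponent stores the given mesh and enables physics simulation on it.
; Each tick it traces along its local down axis and, on a hit, pushes the mesh along its up vector using compression and its rate of change.
; Hits also set the mesh's linear and angular damping.
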(event Custom|InitComponent
  (params (MeshComponent :type Static%20Mesh%20Component%20Object%20Reference))
  (bind _output_get (Variables|Default|SetParentComponent MeshComponent))
  (Physics|SetSimulatePhysics _output_get true))

(event EventTick
  (params (DeltaSeconds :type Float%20%28single-precision%29))
  (bind _returnvalue (Transformation|GetWorldLocation))
  (bind _parentcomponent (Variables|Default|GetParentComponent))
  (bind (_outhit _returnvalue_2) (Collision|LineTraceByChannel _returnvalue (- _returnvalue (* (Math|Vector|GetUpVector) (Variables|Default|GetTraceRange))) "TraceTypeQuery1" false 0 "ForOneFrame"))
  (if _returnvalue_2
    (bind _output_get (Variables|Default|SetHoverDelta (- (Variables|Default|GetTraceRange) (.Distance (Collision|BreakHitResult _outhit)))))
    (Class|PrimitiveComponent|AddForceatLocation _parentcomponent (* (Math|Vector|GetUpVector) (+ (* (/ (- _output_get (Variables|Default|GetPreviousHoverDelta)) (Utilities|Time|GetWorldDeltaSeconds)) (Variables|Default|GetDampingCoefficient)) (* _output_get (Variables|Default|GetSpringCoefficient)))) (Transformation|GetWorldLocation) "None")
    (Class|PrimitiveComponent|SetAngularDamping _parentcomponent 4.0)
    (Class|PrimitiveComponent|SetLinearDamping _parentcomponent 0.8)
    (Variables|Default|SetPreviousHoverDelta (Variables|Default|GetHoverDelta))))